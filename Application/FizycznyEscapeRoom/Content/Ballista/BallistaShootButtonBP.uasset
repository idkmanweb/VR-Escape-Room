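; Interactable button actor that fires the level's ballistas, with a timed cooldown between shots.
; When interacted with while ready, it calls Shoot on all Ballista and Target actors found by class, then starts a reload timer that re-arms it.
; A dynamic material instance on the cylinder shows readiness, red when ready and dark grey while reloading.
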(event `self.ReceiveBeginPlay`
  (bind _returnvalue (`PrimitiveComponent.CreateDynamicMaterialInstance` (`self.Cylinder`) 0 "/Game/Blacksmith/ArrowMaterial.ArrowMaterial" "ButtonMaterial"))
  (bind _output_get (set `self.Material` _returnvalue))
  (`MaterialInstanceDynamic.SetVectorParameterValue` _output_get "Color" (make `LinearColor` 0.9 0.1 0.1 1.0)))

(event `self.Interact`
  (params (HitComponent :type "PrimitiveComponent Object Reference"))
  (if (`self.Ready`)
    (`KismetSystemLibrary.K2_SetTimerDelegate` (delegate `Reload`) 5.0)
    (set `self.Ready` false)
    (`MaterialInstanceDynamic.SetVectorParameterValue` (`self.Material`) "Color" (make `LinearColor` 0.25 0.25 0.25 1.0))
    (bind _outactors (`GameplayStatics.GetAllActorsOfClass` "/Game/Ballista/Ballista.Ballista_C"))
    (`/Game/Ballista/ShootInterface.Shoot` _outactors)
    (bind _outactors_2 (`GameplayStatics.GetAllActorsOfClass` "/Game/Ballista/Target.Target_C"))
    (`/Game/Ballista/ShootInterface.Shoot` _outactors_2)
    (`KismetSystemLibrary.PrintString` "Shooting" true true (struct :`R` 1.0 :`B` 0.139431 :`A` 1.0))))

(event `Reload`
  (set `self.Ready` true)
  (`MaterialInstanceDynamic.SetVectorParameterValue` (`self.Material`) "Color" (make `LinearColor` 0.9 0.2 0.2 1.0)))

(fn `UserConstructionScript`)