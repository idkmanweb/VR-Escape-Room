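; Pointer actor that turns DTrack flystick buttons, read through Live Link, into player actions.
; Each Live Link update compares button states against a cached array to act only on changes.
; Button 0 injects IA_Interact into Enhanced Input and swaps the cube's material; button 1 applies an interpolated yaw step toward 90 degrees.
; Other buttons are empty stubs, and the positioning and line-trace interaction logic is disconnected.
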(event `self.ReceiveBeginPlay`
  (`self.SetActorEnableCollision` false)
  (bind _asbp_architect (cast `/Game/Bridge/BP_Architect` (`GameplayStatics.GetPlayerCharacter` 0)))
  (set `self.As BP Architect` _asbp_architect))

(event `self.ReceiveTick`
  (params (DeltaSeconds :type "Float (single-precision)")))

(event `self.Input.OnLiveLinkUpdated`
  (params (DeltaTime :type "Float (single-precision)"))
  (bind _buttonstate_1 (`self.ButtonState_1`))
  (bind _cube (`self.Cube`))
  (bind _returnvalue (`self.K2_GetActorRotation` (`GameplayStatics.GetPlayerCharacter` 0)))
  (bind _dataresult (`|EvaluateLiveLinkFrameWithSpecificRole` (struct :`Name` "DTrack-FlystickInput-00") "/Script/DTrackPlugin.DTrackFlystickInputRole")
    (:`then`
      (for (_array_element _array_index) (break `DTrackFlystickInputFrameData` (`.m_frame_data` (break `DTrackFlystickInputBlueprintData` _dataresult)))
        (if (!= _array_element (`|GetArrayItem` _buttonstate_1 _array_index))
          (`KismetArrayLibrary.Array_Set` _buttonstate_1 _array_index _array_element)
          (switch `int` _array_index
            (:`0`
              (if _array_element
                (`self.PressedReleassed_Interact` :!label _label
                  (:`Out_Pressed`
                    (`PrimitiveComponent.SetMaterial` _cube 0 "/Game/CAVE/M_SphereCollision.M_SphereCollision"))
                  (:`Out_released`
                    (`PrimitiveComponent.SetMaterial` _cube 0 "/Game/CAVE/M_SphereNoCollision.M_SphereNoCollision")))
                (else
                  (goto _label :!via `released`))))
            (:`1`
              (if _array_element
                (`Controller.SetControlRotation` (`GameplayStatics.GetPlayerController` 0) (`KismetMathLibrary.RInterpTo` _returnvalue (`KismetMathLibrary.MakeRotator` 0.0 0.0 (+ (.yaw _returnvalue) 90.0)) (`GameplayStatics.GetWorldDeltaSeconds`)))
                (`KismetSystemLibrary.PrintString` "Rotated")))
            (:`2`
              (if _array_element
                _))
            (:`3`
              (if _array_element
                _))
            (:`4`
              (if _array_element
                _))
            (:`5`
              (if _array_element
                _))))))))

(fn `UserConstructionScript`)