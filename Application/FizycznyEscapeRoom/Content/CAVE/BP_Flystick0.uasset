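; BP_Flystick0 is a CAVE Flystick actor with a LiveLink input component and a hand collision component.
; Hand overlaps beginning or ending with components whose first tag is "collider" set the Sphere's material, with no material asset specified in either call.
; The LiveLink update event is empty.
; A disconnected, never-run loop detects button changes against a cached state array, with empty per-button branches.
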(event `self.LiveLink_Input.OnLiveLinkUpdated`
  (params (DeltaTime :type "Float (single-precision)")))

(event `self.Hand_colition.OnComponentBeginOverlap`
  (params (OverlappedComponent :type "PrimitiveComponent Object Reference") (OtherActor :type "Actor Object Reference") (OtherComp :type "PrimitiveComponent Object Reference") (OtherBodyIndex :type Integer) (bFromSweep :type Boolean) (SweepResult :type "HitResult Structure (by ref)"))
  (if (== (`|GetArrayItem` (`ActorComponent.ComponentTags` OtherComp)) "collider")
    (`PrimitiveComponent.SetMaterial` (`self.Sphere`) 0 null)))

(event `self.Hand_colition.OnComponentEndOverlap`
  (params (OverlappedComponent :type "PrimitiveComponent Object Reference") (OtherActor :type "Actor Object Reference") (OtherComp :type "PrimitiveComponent Object Reference") (OtherBodyIndex :type Integer))
  (if (== (`|GetArrayItem` (`ActorComponent.ComponentTags` OtherComp)) "collider")
    (`PrimitiveComponent.SetMaterial` (`self.Sphere`) 0 null)))

(fn `UserConstructionScript`)