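; BP_Particle is an interactable particle actor that reports its X, Y and Z values to a Spawner.
; On Interact it prints a debug "Hello" and passes those values to the Spawner's FixAtom.
; GetXYZ exposes the same values, and BeginPlay records the actor's starting location.
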(event `self.ReceiveBeginPlay`
  (set `self.InitialLocation` (`self.K2_GetActorLocation`)))

(event `/Game/InteractInterface.Interact`
  (params (HitComponent :type "PrimitiveComponent Object Reference"))
  (`KismetSystemLibrary.PrintString` "Hello")
  (`/Game/Wizard/BP_ParticleSpawner.FixAtom` (`self.Spawner`) (`self.X`) (`self.Y`) (`self.Z`)))

(fn `GetXYZ`
  (returns (X :type Integer) (Y :type Integer) (Z :type Integer))
  (return (`self.X`) (`self.Y`) (`self.Z`)))

(fn `UserConstructionScript`)