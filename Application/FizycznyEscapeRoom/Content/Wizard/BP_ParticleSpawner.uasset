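; Spawns a cubic lattice of particles at BeginPlay, randomly choosing normal, heavy or inexisting types, stored in a flattened 3D array.
; Each particle is offset from its initial location along the six axes by its neighbours' PreferredDistance.
; FixAtom respawns a cell with a newly random type and reruns the pass through UpdateParticles.
; Prints FINISH when the Finish flag survives every particle's IsOk check.
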(event `self.ReceiveBeginPlay`
  (for _index (range (`self.Size`))
    (for _index_2 (range (`self.Size`))
      (for _index_3 (range (`self.Size`))
        (`self.SpawnParticle` _index_3 _index_2 _index 7))))
  (for _array_element (`self.Particles`) :!label _label
    (`/Engine/EditorBlueprintResources/StandardMacros.IsValid` _array_element
      (:`Is Valid`
        (if (not (`/Game/Wizard/BP_Particle.IsOk` _array_element))
          (set `self.Finish?` false))
        (bind _newparam4 (`self.CalculateOffset` (0.0 0.0 0.0) 1 0 0 _array_element))
        (bind _newparam4_2 (`self.CalculateOffset` _newparam4 -1 0 0 _array_element))
        (bind _newparam4_3 (`self.CalculateOffset` _newparam4_2 0 1 0 _array_element))
        (bind _newparam4_4 (`self.CalculateOffset` _newparam4_3 0 -1 0 _array_element))
        (bind _newparam4_5 (`self.CalculateOffset` _newparam4_4 0 0 1 _array_element))
        (bind _newparam4_6 (`self.CalculateOffset` _newparam4_5 0 0 -1 _array_element))
        (`self.K2_SetActorLocation` _array_element (+ _newparam4_6 (`/Game/Wizard/BP_Particle.InitialLocation` _array_element)) false false))))
  (if (`self.Finish?`)
    (`KismetSystemLibrary.PrintString` "FINISH" true true (struct :`R` 1.0 :`G` 0.898035 :`A` 1.0) 2222.0)))

(event `self.ReceiveTick`
  (params (DeltaSeconds :type "Float (single-precision)")))

(event `UpdateParticles`
  (set `self.Finish?` true)
  (goto _label))

(event `FixAtom`
  (params (NewParam :type Integer) (NewParam2 :type Integer) (NewParam3 :type Integer))
  (bind _newparam (`self.GetParticle` NewParam NewParam2 NewParam3))
  (`self.K2_DestroyActor` _newparam)
  (`self.SpawnParticle` NewParam NewParam2 NewParam3 1)
  (`self.UpdateParticles`))

(fn `CalculateOffset`
  (params (Init :type "Vector Structure") (X :type Integer) (Y :type Integer) (Z :type Integer) (Particle :type "/Game/Wizard/BP_Particle Object Reference"))
  (returns (NewParam4 :type "Vector Structure"))
  (bind (_x _y _z) (`/Game/Wizard/BP_Particle.GetXYZ` Particle))
  (bind _newparam (`self.GetParticle` (+ _x X) (+ Y _y) (+ Z _z)))
  (`/Engine/EditorBlueprintResources/StandardMacros.IsValid` _newparam
    (:`Is Valid`
      (return (+ Init (* (`KismetMathLibrary.MakeVector` (`KismetMathLibrary.Conv_IntToDouble` X) (`KismetMathLibrary.Conv_IntToDouble` Y) (`KismetMathLibrary.Conv_IntToDouble` Z)) (`/Game/Wizard/BP_Particle.PreferredDistance` _newparam) -1.0))))
    (:`Is Not Valid`
      (return Init))))

(fn `GetIndex`
  (params (X :type Integer) (Y :type Integer) (Z :type Integer))
  (returns (NewParam3 :type Integer))
  (return (+ X (* Y (`self.Size`)) (* Z (* (`self.Size`) (`self.Size`))))))

(fn `GetParticle`
  (params (X :type Integer) (Y :type Integer) (Z :type Integer))
  (returns (NewParam :type "/Game/Wizard/BP_Particle Object Reference"))
  (bind _output (`|GetArrayItem` (`self.Particles`) (+ X (* Y (`self.Size`)) (* Z (* (`self.Size`) (`self.Size`))))))
  (bind (_x _y _z) (`/Game/Wizard/BP_Particle.GetXYZ` _output))
  (`/Engine/EditorBlueprintResources/StandardMacros.IsValid` _output
    (:`Is Valid`
      (if (and (== _x X) (== _y Y) (== _z Z))
        (return _output)
        (else
          _)))
    (:`Is Not Valid`
      _))
  (return null))

(fn `GetParticleVector`
  (params (NewParam :type "Vector Structure"))
  (returns (NewParam1 :type "/Game/Wizard/BP_Particle Object Reference"))
  (bind _newparam (`self.GetParticle` (`KismetMathLibrary.FTrunc` NewParam_X) (`KismetMathLibrary.FTrunc` NewParam_Y) (`KismetMathLibrary.FTrunc` NewParam_Z)))
  (return _newparam))

(fn `SpawnParticle`
  (params (NewParam1 :type Integer) (NewParam2 :type Integer) (NewParam3 :type Integer) (Random :type Integer))
  (bind _newparam3 (`self.GetIndex` NewParam1 NewParam2 NewParam3))
  (bind _returnvalue (`|SpawnActorFromClass` (castclass `/Game/Wizard/BP_Particle` (`KismetMathLibrary.SelectClass` "/Game/Wizard/BP_Particle.BP_Particle_C" (`KismetMathLibrary.SelectClass` "/Game/Wizard/BP_HeavyParticle.BP_HeavyParticle_C" "/Game/Wizard/BP_Inexisting.BP_Inexisting_C" (`KismetMathLibrary.RandomBool`)) (`KismetMathLibrary.RandomBoolWithWeight` 0.9)) :!pure true) (`KismetMathLibrary.MakeTransform` (+ (`KismetMathLibrary.MakeVector` (`KismetMathLibrary.Conv_IntToDouble` (* NewParam1 (`self.InitialDistance`))) (`KismetMathLibrary.Conv_IntToDouble` (* NewParam2 (`self.InitialDistance`))) (`KismetMathLibrary.Conv_IntToDouble` (* NewParam3 (`self.InitialDistance`)))) (`self.K2_GetActorLocation`))) "Undefined" "MultiplyWithRoot" null NewParam1 NewParam2 NewParam3 self null))
  (`KismetArrayLibrary.Array_Set` (`self.Particles`) _newparam3 _returnvalue true)
  (`KismetSystemLibrary.PrintString` (`KismetStringLibrary.Conv_IntToString` _newparam3) true true (struct :`G` 0.66 :`B` 1.0 :`A` 1.0) 200.0))

(fn `UserConstructionScript`)