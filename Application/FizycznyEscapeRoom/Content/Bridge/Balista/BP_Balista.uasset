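; BP_Balista is a ballista actor in the Bridge game folder that drives forward once its Started flag is set.
; Tick feeds the forward vector into its Movement component while Started is true.
; ResetPosition restores the transform saved at BeginPlay, toggling capsule physics off and on around the move, and clears Started.
; Mesh hits and FrontRight overlaps only print the other actor's name for debugging.
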(event `self.ReceiveBeginPlay`
  (set `self.InitialPosition` (`self.GetTransform`)))

(event `self.ReceiveTick`
  (params (DeltaSeconds :type "Float (single-precision)"))
  (if (`self.Started`)
    (`PawnMovementComponent.AddInputVector` (`self.Movement`) (`self.GetActorForwardVector`) false)))

(event `self.Mesh.OnComponentHit`
  (params (HitComponent :type "PrimitiveComponent Object Reference") (OtherActor :type "Actor Object Reference") (OtherComp :type "PrimitiveComponent Object Reference") (NormalImpulse :type "Vector Structure") (Hit :type "HitResult Structure (by ref)"))
  (`KismetSystemLibrary.PrintString` (`KismetSystemLibrary.GetDisplayName` OtherActor)))

(event `self.FrontRight.OnComponentBeginOverlap`
  (params (OverlappedComponent :type "PrimitiveComponent Object Reference") (OtherActor :type "Actor Object Reference") (OtherComp :type "PrimitiveComponent Object Reference") (OtherBodyIndex :type Integer) (bFromSweep :type Boolean) (SweepResult :type "HitResult Structure (by ref)"))
  (`KismetSystemLibrary.PrintString` (`KismetSystemLibrary.GetDisplayName` OtherActor) true true (struct :`G` 1.0 :`B` 0.388788 :`A` 1.0)))

(fn `ResetPosition`
  (`PrimitiveComponent.SetSimulatePhysics` (`self.Capsule`) false)
  (`self.K2_SetActorTransform` (`self.InitialPosition`))
  (`PrimitiveComponent.SetSimulatePhysics` (`self.Capsule`) true)
  (set `self.Started` false))

(fn `UserConstructionScript`)